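; Stat-boost orb pickup that homes in on the player character and calls StatsUp with its StatsUpType on bp_thirdperson when within 10 units.
; Each tick it moves toward a point below the player's origin, accelerating to a capped speed and shrinking with distance inside 100 units.
; Movement requires a positive Timer, which BeginPlay zeroes and nothing here raises.
; DestroyActor is unwired, so the orb never destroys itself.
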(event `self.ReceiveTick`
  (params (DeltaSeconds :type "Float (single-precision)"))
  (`self.Movement Tick`))

(event `self.ReceiveBeginPlay`
  ;[1 1 1] Move to player and Pickup
  (bind _asbp_thirdperson (cast `/Game/bp/bp_thirdperson` (`GameplayStatics.GetPlayerCharacter` 0)))
  (set `self.Teddy` _asbp_thirdperson)
  (set `self.Timer` 0.0))

(event `Movement Tick`
  (bind _returnvalue (- (`KismetMathLibrary.MakeVector` (.x (`self.K2_GetActorLocation` (`GameplayStatics.GetPlayerCharacter` 0))) (.y (`self.K2_GetActorLocation` (`GameplayStatics.GetPlayerCharacter` 0))) (- (.z (`self.K2_GetActorLocation` (`GameplayStatics.GetPlayerCharacter` 0))) 40.0)) (`SceneComponent.K2_GetComponentLocation` (`self.orb`))))
  (bind _returnvalue_2 (`KismetMathLibrary.VSize` _returnvalue))
  ;[1 1 1] Move to player and Pickup
  (if (not (<= (`self.Timer`) 0.0))
    (if (< _returnvalue_2 100.0)
      (set `self.movement speed` (`KismetMathLibrary.FMin` (+ (`self.movement speed`) (`self.acceleration`)) (`self.max movement speed`))))
    (if (< _returnvalue_2 100.0)
      (set `self.new scale` (* (0.25 0.25 0.25) (/ _returnvalue_2 100.0))))
    (`SceneComponent.K2_SetWorldTransform` (`self.orb`) (`KismetMathLibrary.MakeTransform` (+ (`SceneComponent.K2_GetComponentLocation` (`self.orb`)) (* (`KismetMathLibrary.Normal` _returnvalue) (`self.movement speed`))) (struct) (`self.new scale`)) false false)
    (if (< (`KismetMathLibrary.VSize` _returnvalue) 10.0)
      (`/Game/bp/bp_thirdperson.StatsUp` (`self.Teddy`) (`self.Stats Up Type`)))))

(fn `UserConstructionScript`)