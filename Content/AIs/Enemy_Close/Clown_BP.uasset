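; Clown_BP is a close-range clown enemy that attacks the player with a mace.
; MeleeAttack calls MaceTracing, plays a single attack animation, then immediately disables RightMace collision.
; MaceTracing enables that collision and sphere-traces forward from the mace with persistent debug drawing, applying damage and spawning a zero-scaled explosion emitter on player hits.
; The IsAttacking guard, montage playback and random attack pick are disconnected.
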(event `MeleeAttack`
  (switch `int` 0
    (:`0`
      (`self.Mace Tracing`)
      (`SkeletalMeshComponent.PlayAnimation` (`self.Mesh`) "/Game/Mannequin/Animations/Clown/Clown_Animation_Normal01.Clown_Animation_Normal01" false)
      (`PrimitiveComponent.SetCollisionEnabled` (`self.RightMace`) "NoCollision"))))

(event `Mace Tracing`
  (bind _rightmace (`self.RightMace`))
  (bind _returnvalue (`SceneComponent.K2_GetComponentLocation` _rightmace))
  (`PrimitiveComponent.SetCollisionEnabled` _rightmace "QueryAndPhysics")
  (bind (_outhit _returnvalue_2) (`KismetSystemLibrary.SphereTraceSingle` :`Start` _returnvalue :`End` (+ _returnvalue (* (`KismetMathLibrary.GetForwardVector` (`SceneComponent.K2_GetComponentRotation` _rightmace)) 1000.0)) :`Radius` 65.0 :`TraceChannel` "TraceTypeQuery1" :`DrawDebugType` "Persistent"))
  (if _returnvalue_2
    (bind (_bblockinghit _binitialoverlap _time _distance _location _impactpoint _normal _impactnormal _physmat _hitactor) (`GameplayStatics.BreakHitResult` _outhit))
    (if (== _hitactor (`GameplayStatics.GetPlayerCharacter` 0))
      (bind _returnvalue_3 (`GameplayStatics.SpawnEmitterAtLocation` "/Game/StarterContent/Particles/P_Explosion.P_Explosion" _location))
      (`SceneComponent.SetWorldScale3D` _returnvalue_3 (0.0 0.0 0.0))
      (`GameplayStatics.ApplyDamage` _hitactor 10.0 (`self.GetController`) self))))

(fn `UserConstructionScript`)